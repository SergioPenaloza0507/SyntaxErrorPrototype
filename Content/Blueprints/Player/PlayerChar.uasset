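; Player character Blueprint that handles camera-relative movement from the Vertical and Horizontal input axes.
; Both axis events share one AddInputVector call on the CharacterMovement component.
; The movement vector sums the camera's forward and right vectors, each flattened onto the horizontal plane and scaled by an axis value.
; BeginPlay, overlap, Tick and the construction script are empty.
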(event `InputAxis|Vertical`
  (params (AxisValue :type "Float (single-precision)"))
  (bind _camera (`self.Camera`))
  (`PawnMovementComponent.AddInputVector` (`self.CharacterMovement`) (+ (* (`KismetMathLibrary.ProjectVectorOnToPlane` (`SceneComponent.GetForwardVector` _camera) (0.0 0.0 1.0)) AxisValue) (* (`KismetMathLibrary.ProjectVectorOnToPlane` (`SceneComponent.GetRightVector` _camera) (0.0 0.0 1.0)) (stale `InputAxis|Horizontal` AxisValue))) false :!label _label))

(event `InputAxis|Horizontal`
  (params (AxisValue :type "Float (single-precision)"))
  (goto _label))

(fn `UserConstructionScript`)